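; BP_BulletProjectile is a bullet projectile that damages actors its Box collision overlaps, excluding the instigator who fired it.
; On BeginPlay the Box ignores the instigator when moving, and the overlap handler also checks against it.
; A valid overlap applies the Damage variable to the other actor and spawns an emitter at the Box's location.
; The graph does not destroy the bullet after a hit.
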(event `self.ReceiveBeginPlay`
  ;[1 1 1] Prevent Overlaping with the Player who Fired it
  (`PrimitiveComponent.IgnoreActorWhenMoving` (`self.Box`) (`self.GetInstigator`) true))

(event `self.Box.OnComponentBeginOverlap`
  (params (OverlappedComponent :type "PrimitiveComponent Object Reference") (OtherActor :type "Actor Object Reference") (OtherComp :type "PrimitiveComponent Object Reference") (OtherBodyIndex :type Integer) (bFromSweep :type Boolean) (SweepResult :type "HitResult Structure (by ref)"))
  (if (!= OtherActor (`self.GetInstigator`))
    (`GameplayStatics.ApplyDamage` OtherActor (`self.Damage`))
    (`GameplayStatics.SpawnEmitterAtLocation` null (`SceneComponent.K2_GetComponentLocation` (`self.Box`)))))

(fn `UserConstructionScript`)