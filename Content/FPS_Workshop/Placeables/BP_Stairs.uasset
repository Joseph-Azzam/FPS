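; Placeable climbing volume that lets the player soldier move up and down on stairs.
; Construction script sizes and centers the box from VolumeExtent and a Z-only EndLocation.
; Box overlap switches the player to Flying with braking to prevent drift, restoring Walking on exit.
; While inside, Tick compares camera pitch against MoveAngle, setting UsingStairs for vertical movement and inverting forward input when looking down.
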(event `self.ReceiveTick`
  (params (DeltaSeconds :type "Float (single-precision)"))
  (bind _moveangle (`self.MoveAngle`))
  (bind _player (`self.Player`))
  (bind _returnvalue (`KismetMathLibrary.Dot_VectorVector` (`KismetMathLibrary.Conv_RotatorToVector` (`SceneComponent.K2_GetComponentRotation` (`/Game/FPS_Workshop/Core/BP_Soldier_Character.FirstPersonCamera` (`self.Player`)))) (`self.LookUpVector`)))
  (bind _returnvalue_2 (<= _returnvalue (* _moveangle -1.0)))
  (if (`self.bPlayerInside`)
    (set `/Game/FPS_Workshop/Core/BP_Soldier_Character.bUsingStairs` (or (>= _returnvalue _moveangle) _returnvalue_2) _player) ; Change the Player Movement to Up/Dow instead of Left Right
    (set `/Game/FPS_Workshop/Core/BP_Soldier_Character.bInvertForwardMovement` _returnvalue_2 _player) ; Invert the Player Movement if the player is looking down
  ))

(event `self.Box.OnComponentBeginOverlap`
  (params (OverlappedComponent :type "PrimitiveComponent Object Reference") (OtherActor :type "Actor Object Reference") (OtherComp :type "PrimitiveComponent Object Reference") (OtherBodyIndex :type Integer) (bFromSweep :type Boolean) (SweepResult :type "HitResult Structure (by ref)"))
  (bind _charactermovement (`Character.CharacterMovement` (`self.Player`)))
  ;[1 1 1] Check if the Player Entered
  (if (== OtherActor (`GameplayStatics.GetPlayerCharacter` 0))
    ;[1 1 1] Save a Reference to the Player
    (bind _asbp_soldier_character (cast `/Game/FPS_Workshop/Core/BP_Soldier_Character` OtherActor))
    (set `self.Player` _asbp_soldier_character)
    (set `self.bPlayerInside` true)
    ;[1 1 1] Enable the Plaer to Walk/Fly
    (`CharacterMovementComponent.SetMovementMode` _charactermovement "MOVE_Flying" 0)
    (set `CharacterMovementComponent.BrakingDecelerationFlying` 1000.0 _charactermovement) ; Disable Player Drifting while Flying
  ))

(event `self.Box.OnComponentEndOverlap`
  (params (OverlappedComponent :type "PrimitiveComponent Object Reference") (OtherActor :type "Actor Object Reference") (OtherComp :type "PrimitiveComponent Object Reference") (OtherBodyIndex :type Integer))
  (bind _player (`self.Player`))
  (bind _charactermovement (`Character.CharacterMovement` (`self.Player`)))
  ;[1 1 1] Clear the Player
  (bind _asbp_soldier_character (cast `/Game/FPS_Workshop/Core/BP_Soldier_Character` OtherActor))
  (set `self.bPlayerInside` (not (== _asbp_soldier_character (`self.Player`))))
  ;[1 1 1] Enable the Plaer to Walk/Fly
  (`CharacterMovementComponent.SetMovementMode` _charactermovement "MOVE_Walking" 0)
  (set `CharacterMovementComponent.BrakingDecelerationFlying` 0.0 _charactermovement) ; Re-Enable Player Drifting while Flying
  ;[1 1 1] Reset Variables
  (set `/Game/FPS_Workshop/Core/BP_Soldier_Character.bUsingStairs` false _player)
  (set `/Game/FPS_Workshop/Core/BP_Soldier_Character.bInvertForwardMovement` false _player)
  (set `self.Player` null))

(fn `UserConstructionScript`
  (bind _box (`self.Box`))
  (bind (_endlocation_x _endlocation_y _endlocation_z) (`KismetMathLibrary.BreakVector` (`self.EndLocation`)))
  (bind (_volumeextent_x _volumeextent_y) (`KismetMathLibrary.BreakVector2D` (`self.VolumeExtent`)))
  (bind _z (.z (`self.EndLocation`)))
  (bind _returnvalue (/ _endlocation_z 2.0))
  ;[1 1 1] Lock X and Y Axis for Locations
  (set `self.EndLocation` (`KismetMathLibrary.MakeVector` 0.0 0.0 (select `bool` (<= _z 0.0) :`false` _z)))
  ;[1 1 1] Set Box Size and Location
  (`BoxComponent.SetBoxExtent` _box (`KismetMathLibrary.MakeVector` _volumeextent_x _volumeextent_y _returnvalue) true)
  (`SceneComponent.K2_SetRelativeLocation` _box (`KismetMathLibrary.MakeVector` 0.0 0.0 _returnvalue) false false))